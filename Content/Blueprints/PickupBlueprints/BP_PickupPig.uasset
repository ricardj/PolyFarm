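; BP_PickupPig is a pickup actor that BP_MotionController can grab and hold.
; Pickup disables mesh physics, snaps the root to the supplied component, then shrinks and tilts the mesh with a hand-tuned relative offset.
; Drop detaches the actor in world space, restores full mesh scale, resets the mesh's relative transform to a raised offset and re-enables physics.
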(event EventBeginPlay)

(event Collision|EventActorBeginOverlap
  (params (OtherActor :type Actor%20Object%20Reference)))

(event EventTick
  (params (DeltaSeconds :type Float%20%28single-precision%29)))

(event EventPickup
  (params (AttachTo :type Scene%20Component%20Object%20Reference))
  (bind _staticmeshcomponent (Variables|Debug|GetStaticMeshComponent))
  (Physics|SetSimulatePhysics (Variables|Debug|GetStaticMeshComponent) false)
  (Transformation|AttachComponentToComponent (VehicleSound|GetRootComponent) AttachTo "None" "SnapToTarget" "SnapToTarget" "SnapToTarget" false)
  (Transformation|SetRelativeLocationAndRotation _staticmeshcomponent "3.726645,6.847500,-0.997499" "0, 0,-60.000114" false false)
  (Transformation|SetRelativeScale3D _staticmeshcomponent "0.094578,0.094578,0.094578"))

(event EventDrop
  (bind _staticmeshcomponent (Variables|Debug|GetStaticMeshComponent))
  (Transformation|DetachFromActor "KeepWorld" "KeepWorld" "KeepWorld")
  (Transformation|SetRelativeScale3D _staticmeshcomponent "1.000000,1.000000,1.000000")
  (Transformation|SetRelativeLocationAndRotation _staticmeshcomponent "0,0.000000,50.000000" "0, 0, 0" false false)
  (Physics|SetSimulatePhysics (Variables|Debug|GetStaticMeshComponent) true))

(fn ConstructionScript)