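; Tutorial portal trigger that sends the game to the polyFarm level when the correct object enters it.
; On overlap it reads the OpenPortal flag from the tutorial_escena game instance and reacts only while that is set.
; A "sphere"-tagged actor is destroyed, then a success sound plays before the delayed level load.
; Other actors trigger a wrong-answer sound, throttled by the game instance's Sound flag and a delay.
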(event EventBeginPlay)

(event Collision|EventActorBeginOverlap
  (params (OtherActor :type Actor%20Object%20Reference))
  (Utilities|FlowControl|Sequence
    (:then_0
      (bind _astutorial_escena (Utilities|Casting|CastTotutorial_escena (Game|GetGameInstance))
        (:CastFailed
          (Development|PrintString "Hello"))))
    (:then_1
      (if (Variables|/Game/Blueprints/scene/tutorial_escena.tutorial_escena_C|GetopenPortal _astutorial_escena)
        (if (Utilities|Array|ContainsItem (Variables|/Script/Engine.Actor|GetTags OtherActor) "sphere")
          (Actor|DestroyActor OtherActor)
          (Audio|PlaySoundatLocation "/Game/audios/muyBienHemosLLegado_Cue.muyBienHemosLLegado_Cue" "0, 0, 0" "0, 0, 0" 1.0 1.0 0.0 0 0 0)
          (Utilities|FlowControl|Delay 5.5)
          (Game|OpenLevel(byName) "polyFarm")
          (else
            (Utilities|FlowControl|Sequence
              (:then_0
                (if (not (Variables|/Game/Blueprints/scene/tutorial_escena.tutorial_escena_C|Getsound _astutorial_escena))
                  (Variables|/Game/Blueprints/scene/tutorial_escena.tutorial_escena_C|Setsound _astutorial_escena true)
                  (Audio|PlaySoundatLocation "/Game/audios/tutorial/respuesta_incorrecta_Cue.respuesta_incorrecta_Cue" "0, 0, 0" "0, 0, 0" 1.0 1.0 0.0 0 0 0)
                  (Utilities|FlowControl|Delay 4.0)
                  (Variables|/Game/Blueprints/scene/tutorial_escena.tutorial_escena_C|Setsound _astutorial_escena false))))))))))

(event EventTick
  (params (DeltaSeconds :type Float%20%28single-precision%29)))

(fn ConstructionScript)