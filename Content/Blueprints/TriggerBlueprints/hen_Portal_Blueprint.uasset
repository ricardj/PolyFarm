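; Tutorial portal trigger that consumes actors tagged "hen" and counts its own completion once.
; On overlap it debug-prints the actor's name, then destroys a tagged hen with a particle burst and swoosh.
; The first hen increments and checks the counter on the tutorial_escena GameInstance, sets Block, and plays Spanish "go to next portal" praise.
; Later hens only trigger the "already completed" voice line; sounds spawn at world origin.
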(event EventBeginPlay)

(event Collision|EventActorBeginOverlap
  (params (OtherActor :type Actor%20Object%20Reference))
  (Development|PrintString (Utilities|GetObjectName OtherActor) true true "(R=1.000000,G=0.000000,B=0.096778,A=1.000000)")
  (if (Utilities|Array|ContainsItem (Variables|/Script/Engine.Actor|GetTags OtherActor) "hen")
    (Effects|SpawnEmitteratLocation "/Game/InfinityBladeEffects/Effects/FX_Monsters/FX_Monster_Bear/P_Bear_DoubleSlash_01.P_Bear_DoubleSlash_01" (Transformation|GetActorLocation OtherActor))
    (Actor|DestroyActor OtherActor)
    (Audio|SpawnSoundatLocation "/Game/audios/swoosh_v1_Cue.swoosh_v1_Cue" "0, 0, 0" "0, 0, 0" 1.0 1.0 0.0 0 0)
    (if (Variables|Default|Getblock)
      (Audio|SpawnSoundatLocation "/Game/audios/PortalRicard/EstePortalYaEstaCompletado_Cue.EstePortalYaEstaCompletado_Cue" "0, 0, 0" "0, 0, 0" 1.0 1.0 0.0 0 0)
      (else
        (bind _astutorial_escena (Utilities|Casting|CastTotutorial_escena (Game|GetGameInstance)))
        (Variables|/Game/Blueprints/scene/tutorial_escena.tutorial_escena_C|Setcounter _astutorial_escena (+ (Variables|/Game/Blueprints/scene/tutorial_escena.tutorial_escena_C|Getcounter _astutorial_escena) 1))
        (Default|CheckCounterValue _astutorial_escena)
        (Variables|Default|Setblock true)
        (Audio|SpawnSoundatLocation "/Game/audios/PortalRicard/MuyBIenPasaAlsiguientePortal.MuyBIenPasaAlsiguientePortal" "0, 0, 0" "0, 0, 0" 1.0 1.0 0.0 0 0)))))

(event EventTick
  (params (DeltaSeconds :type Float%20%28single-precision%29)))

(fn ConstructionScript)